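; YOSWGmode, apparently a game mode, holds economy state for an IT-center upgrade game and pays passive income.
; BeginPlay seeds the level, starting cash, income amount, interval and a Russian maximum-level message.
; Tick chains two latent Delays, one fixed and one using CashplusperSec, as a repeating timer before adding Cashpluser to Cash.
; Nothing here changes the level or uses the message.
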(event `self.ReceiveBeginPlay`
  (set `self.level` 1)
  (set `self.cashplusper sec` 1.0)
  (set `self.cashpluser` 25.0)
  (set `self.level end` "МАКСИМАЛЬНЫЙ УРОВЕНЬ  IT-ЦЕНТРА")
  (set `self.cash` 10000.0))

(event `self.ReceiveTick`
  (params (DeltaSeconds :type "Float (single-precision)"))
  (`KismetSystemLibrary.Delay` 1.0)
  (`KismetSystemLibrary.Delay` (`self.cashplusper sec`))
  (set `self.cash` (+ (`self.cash`) (`self.cashpluser`))))

(fn `UserConstructionScript`)